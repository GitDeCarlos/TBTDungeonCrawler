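; Player interaction component that lets its owning Character interact with nearby actors implementing BPI_Interactable.
; On BeginPlay it binds to the owner's capsule overlap events, adding interactables to an in-range list on begin overlap and removing them on end overlap.
; The IA_Interact input sends InteractMessage, with the owner as argument, to the first valid entry in that list, with no distance or facing priority.
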(event Custom|HandleOnComponentBeginOverlap
  (params (OverlappedComponent :type Primitive%20Component%20Object%20Reference) (OtherActor :type Actor%20Object%20Reference) (OtherComp :type Primitive%20Component%20Object%20Reference) (OtherBodyIndex :type Integer) (bFromSweep :type Boolean) (SweepResult :type Hit%20Result%20Structure%20%28by%20ref%29))
  (if (Utilities|DoesObjectImplementInterface OtherActor "/Game/Game/Blueprints/Interfaces/BPI_Interactable.BPI_Interactable_C")
    (Utilities|Array|AddUnique (Variables|Default|GetInteractablesInRange) OtherActor)))

(event Custom|HandleOnComponentEndOverlap
  (params (OverlappedComponent :type Primitive%20Component%20Object%20Reference) (OtherActor :type Actor%20Object%20Reference) (OtherComp :type Primitive%20Component%20Object%20Reference) (OtherBodyIndex :type Integer))
  (if (Utilities|DoesObjectImplementInterface OtherActor "/Game/Game/Blueprints/Interfaces/BPI_Interactable.BPI_Interactable_C")
    (Utilities|Array|RemoveItem (Variables|Default|GetInteractablesInRange) OtherActor)))

(event Input|EnhancedActionEvents|EnhancedInputActionIA_Interact
  (params (ActionValue :type Boolean) (ElapsedSeconds :type Float%20%28double-precision%29) (TriggeredSeconds :type Float%20%28double-precision%29) (InputAction :type Input%20Action%20Object%20Reference :default "/Game/Game/Systems/Input/Actions/IA_Interact.IA_Interact"))
  (bind _interactablesinrange (Variables|Default|GetInteractablesInRange))
  (bind _output (Utilities|Array|Get(acopy) _interactablesinrange))
  ;[0.15 0.15 0.15 0.5] Handle input for interact
  (:Started
    (Utilities|IsValid _output
      (:Is%20Valid
        (Class|BPIInteractable|Interact(Message) _output (Components|GetOwner))))))

(event EventBeginPlay
  (bind _ascharacter (Utilities|Casting|CastToCharacter (Components|GetOwner)))
  (Collision|BindEventtoOnComponentBeginOverlap (Variables|/Script/Engine.Character|GetCapsuleComponent _ascharacter) (EventDispatchers|CreateEvent :!event Custom|HandleOnComponentBeginOverlap))
  (Collision|BindEventtoOnComponentEndOverlap (Variables|/Script/Engine.Character|GetCapsuleComponent _ascharacter) (EventDispatchers|CreateEvent :!event Custom|HandleOnComponentEndOverlap)))