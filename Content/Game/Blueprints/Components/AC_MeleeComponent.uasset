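; Actor component that gives its owner a melee attack by line trace, damaging the actor it hits.
; MeleeAttack traces from the player's camera, or from the owner's location and facing when no camera is cached, firing hit, damaged or missed callbacks.
; Successful damage also raises an AI damage sense report.
; An optional TBTTimer drives a cooldown flag, started and queried separately because the attack itself does not check it.
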(event Custom|MeleeAttack
  (bind _returnvalue (Components|GetOwner))
  ;[0.15 0.15 0.15 0.5] Attack line trace
  (Utilities|FlowControl|Sequence
    (:then_0
      (bind (_startlocation _endlocation) (CallFunction|GetLineTraceLocationsfromCamera))
      (bind (_outhit _returnvalue_2) (Collision|LineTraceByChannel _startlocation _endlocation "TraceTypeQuery1" false 0 (Variables|Parameters|GetLineDrawDebugType) true "(R=1.000000,G=0.000356,B=0.096022,A=1.000000)"))
      (if _returnvalue_2
        (Default|CallOnTargetHit _outhit)
        (bind _success (CallFunction|TryApplyDamage (.HitActor (Collision|BreakHitResult _outhit)) (Variables|Parameters|GetDamagePoints) (Components|GetOwner)))
        (if _success
          (Class|AISenseDamage|ReportDamageEvent (.HitActor (Collision|BreakHitResult _outhit)) _returnvalue 2.0 (Transformation|GetActorLocation _returnvalue) (.Location (Collision|BreakHitResult _outhit)) "None")
          (Default|CallOnTargetDamaged _outhit))
        (else
          (Default|CallOnTargetMissed))))
    (:then_1
      (Utilities|FlowControl|Delay 0.4))))

(event Custom|FinishCooldown
  (Variables|Default|SetIsCooldownActive false))

(event Custom|TryBeginAttackCooldown
  (if (not (Variables|Default|GetIsCooldownActive))
    (Variables|Default|SetIsCooldownActive true)
    (Class|TBTTimer|Start (Variables|Default|GetCooldownTimer))))

(event EventBeginPlay
  (bind _returnvalue (Components|GetOwner))
  (bind _returnvalue_2 (Actor|GetComponentsByClass _returnvalue "/Script/Engine.CameraComponent"))
  (bind _output (Utilities|Array|Get(acopy) _returnvalue_2))
  (Utilities|FlowControl|Sequence
    (:then_0
      ;[1 0.000356 0.09602] Possibly redundant, revisit later
      (bind _output_get (Variables|Default|SetIsPlayer (== (Components|GetOwner) (Game|Player|GetPlayerPawn 0))))
      (if _output_get
        (Utilities|IsValid _output
          (:Is%20Valid
            (Variables|Default|SetOwnerCameraRef _output)))))
    (:then_1
      ;[0.15 0.15 0.15 0.5] Initializing attack cooldown
      (if (Variables|Parameters|GetEnableCooldownTimer)
        (bind _returnvalue_3 (Game|ConstructObjectfromClass "/Script/TBTDungeonCrawler.TBTTimer"))
        (bind _output_get_2 (Variables|Default|SetCooldownTimer _returnvalue_3))
        (Class|TBTTimer|Initialize _output_get_2 self (Variables|Parameters|GetCooldownLength) (CallFunction|GetTickRate))
        (EventDispatchers|BindEventtoOnTimerFinished _output_get_2 (EventDispatchers|CreateEvent :!event Custom|FinishCooldown))))))

(fn GetLineTraceLocationsfromCamera
  (bind _ownercameraref (Variables|Default|GetOwnerCameraRef)
    (:then
      (return (Transformation|GetWorldLocation _ownercameraref) (+ (Transformation|GetWorldLocation _ownercameraref) (* (Math|Vector|GetForwardVector _ownercameraref) (Variables|Parameters|GetMeleeRange)))))
    (:else
      ;[0.15 0.15 0.15 0.5] Default to Owner if camera component not found
      (bind (_startlocation _endlocation) (CallFunction|GetLineTraceLocationsfromOwner))
      (return _startlocation _endlocation))))

(fn GetLineTraceLocationsfromOwner
  (bind _returnvalue (Components|GetOwner))
  (bind _returnvalue_2 (Transformation|GetActorLocation _returnvalue))
  (return _returnvalue_2 (+ _returnvalue_2 (* (Transformation|GetActorForwardVector _returnvalue) (Variables|Parameters|GetMeleeRange)))))

(fn GetIsCooldownActive
  (return (Variables|Default|GetIsCooldownActive)))