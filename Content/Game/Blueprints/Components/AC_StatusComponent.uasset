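; Status component that tracks health and stamina for its owner, broadcasting change, hit, death and stamina-break events.
; Blocked hits drain fixed stamina instead of health, and hits on the player pawn trigger camera shake.
; Damage and stamina drain restart TBTTimer cooldown objects that pair with ticking regen timers, with health regen optional.
; Health regen accumulates progress into rounded heals, using StaminaRegenSpeed as its rate.
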(event Custom|BeginHealthRegenCooldown
  ;[1 0.3419 0.3325] New Health Regen Code
  (Variables|Default|SetHealthProgress 0.0)
  (Class|TBTTimer|Stop (Variables|HealthRegen|GetHealthRegenObject))
  (Class|TBTTimer|Start (Variables|HealthRegen|GetHealthCooldownObject)))

(event Custom|HandleHealthRegen
  (params (TimeElapsed :type Float%20%28double-precision%29))
  ;[1 0.3419 0.3325] New Health Regen Code
  (Variables|Default|SetHealthProgress (+ (Variables|Default|GetHealthProgress) (* (CallFunction|GetTickRate) (Variables|Parameters|GetStaminaRegenSpeed))))
  (if (>= (Variables|Default|GetHealthCurrent) (Variables|Parameters|GetHealthMax))
    (Class|TBTTimer|Stop (Variables|HealthRegen|GetHealthRegenObject))
    (elif (> (Variables|Default|GetHealthProgress) 1.0)
      (CallFunction|Heal (Math|Conversions|ToFloat(Integer) (Math|Float|Round (Variables|Default|GetHealthProgress))))
      (Variables|Default|SetHealthProgress 0.0))))

(event Custom|FinishHealthRegen
  ;[1 0.3419 0.3325] New Health Regen Code
  (if (< (Variables|Default|GetHealthCurrent) (Variables|Parameters|GetHealthMax))
    (CallFunction|BeginHealthRegen)))

(event Custom|BeginStaminaRegenCooldown
  ;[0.2086 0.4179 1] New Stamina Regen Code
  (Class|TBTTimer|Stop (Variables|StaminaRegen|GetStaminaRegenObject))
  (Class|TBTTimer|Start (Variables|StaminaRegen|GetStaminaCooldownObject)))

(event Custom|HandleStaminaRegen
  (params (Time%20Elapsed :type Float%20%28double-precision%29))
  ;[0.2086 0.4179 1] New Stamina Regen Code
  (if (>= (Variables|Default|GetStaminaCurrent) (Variables|Parameters|GetStaminaMax))
    (Class|TBTTimer|Stop (Variables|StaminaRegen|GetStaminaRegenObject))
    (else
      (CallFunction|RestoreStamina (* (CallFunction|GetTickRate) (Variables|Parameters|GetStaminaRegenSpeed))))))

(event Custom|FinishStaminaRegen
  ;[0.2086 0.4179 1] New Stamina Regen Code
  (if (< (Variables|Default|GetStaminaCurrent) (Variables|Parameters|GetStaminaMax))
    (CallFunction|BeginStaminaRegen)))

(event Custom|BeginHealthRegen
  ;[1 0.3419 0.3325] New Health Regen Code
  (Class|TBTTimer|Start (Variables|HealthRegen|GetHealthRegenObject)))

(event Custom|BeginStaminaRegen
  ;[0.2086 0.4179 1] New Stamina Regen Code
  (Class|TBTTimer|Start (Variables|StaminaRegen|GetStaminaRegenObject)))

(event EventApplyDamage
  (params (DamagePoints :type Float%20%28double-precision%29) (Source :type Actor%20Object%20Reference))
  (CallFunction|Damage DamagePoints)
  (CallFunction|BeginHealthRegenCooldown))

(event EventBeginPlay
  (bind _healthmax (Variables|Parameters|GetHealthMax))
  (bind _staminamax (Variables|Parameters|GetStaminaMax))
  (Utilities|FlowControl|Sequence
    (:then_0
      (bind _output_get (Variables|Default|SetHealthCurrent _healthmax))
      (Default|CallOnHealthChanged _output_get _healthmax)
      (bind _output_get_2 (Variables|Default|SetStaminaCurrent _staminamax))
      (Default|CallOnStaminaChanged _output_get_2 _staminamax))
    (:then_1
      (Utilities|FlowControl|Delay 0.2)
      (CallFunction|Heal 1.0)
      (CallFunction|RestoreStamina 1.0))
    (:then_2
      (CallFunction|InitRegenTimers))))

(event EventApplyStaminaDrain
  (params (StaminaPoints :type Float%20%28double-precision%29) (Source :type Actor%20Object%20Reference))
  (CallFunction|DrainStamina StaminaPoints)
  (CallFunction|BeginStaminaRegenCooldown))

(fn Damage
  (params (DamagePoints :type Float%20%28double-precision%29))
  (Default|CallOnHit)
  (if (not (Variables|Default|GetIsBlocking))
    (Utilities|FlowControl|Sequence
      (:then_0
        ;[0.15 0.15 0.15 0.5] Apply damage, dispatch OnHealthChanged, OnReceivedDamage
        (Variables|Default|SetHealthCurrent (Math|Float|Clamp(Float) (- (Variables|Default|GetHealthCurrent) DamagePoints) 0.0 (Variables|Parameters|GetHealthMax)))
        (Default|CallOnHealthChanged (Variables|Default|GetHealthCurrent) (Variables|Parameters|GetHealthMax))
        (Default|CallOnReceivedDamage))
      (:then_1
        ;[0.15 0.15 0.15 0.5] Check if still alive
        (bind _output_get (Variables|Default|SetIsDead (<= (Variables|Default|GetHealthCurrent) 0.0)))
        (if _output_get
          (Default|CallOnDeath)))
      (:then_2
        (if (== (Components|GetOwner) (Game|Player|GetPlayerPawn 0)) :!label _label
          (Camera|PlayWorldCameraShake "/Game/Game/Blueprints/CameraShake/CS_Melee.CS_Melee_C" (Utilities|GetOwnerLocation) 0.0 1e+03))))
    (else
      (CallFunction|DrainStamina 1e+01)
      (goto _label))))

(fn Heal
  (params (HealthPoints :type Float%20%28double-precision%29))
  (Variables|Default|SetHealthCurrent (Math|Float|Clamp(Float) (+ HealthPoints (Variables|Default|GetHealthCurrent)) 0.0 (Variables|Parameters|GetHealthMax)))
  (Default|CallOnHealthChanged (Variables|Default|GetHealthCurrent) (Variables|Parameters|GetHealthMax)))

(fn DrainStamina
  (params (StaminaPoints :type Float%20%28double-precision%29))
  (Variables|Default|SetStaminaCurrent (Math|Float|Clamp(Float) (- (Variables|Default|GetStaminaCurrent) StaminaPoints) 0.0 (Variables|Parameters|GetStaminaMax)))
  (Default|CallOnStaminaChanged (Variables|Default|GetStaminaCurrent) (Variables|Parameters|GetStaminaMax))
  (if (<= (Variables|Default|GetStaminaCurrent) 0.0)
    (Default|CallOnStaminaBreak)))

(fn RestoreStamina
  (params (StaminaPoints :type Float%20%28double-precision%29))
  (Variables|Default|SetStaminaCurrent (Math|Float|Clamp(Float) (+ (Variables|Default|GetStaminaCurrent) StaminaPoints) 0.0 (Variables|Parameters|GetStaminaMax)))
  (Default|CallOnStaminaChanged (Variables|Default|GetStaminaCurrent) (Variables|Parameters|GetStaminaMax)))

(fn GetIsDead
  (return (Variables|Default|GetIsDead)))

(fn SetIsBlocking
  (params (IsBlocking :type Boolean))
  (Utilities|FlowControl|Sequence
    (:then_0
      (if (Variables|Default|GetIsBlocking)
        _))
    (:then_1
      (Variables|Default|SetIsBlocking IsBlocking))))

(fn InitRegenTimers
  (Utilities|FlowControl|Sequence
    (:then_0
      (Utilities|FlowControl|Sequence
        (:then_0
          ;[0.15 0.15 0.15 0.5] Cooldown Timer Object
          (bind _returnvalue (Game|ConstructObjectfromClass "/Script/TBTDungeonCrawler.TBTTimer"))
          (bind _output_get (Variables|HealthRegen|SetHealthCooldownObject _returnvalue))
          (Class|TBTTimer|Initialize _output_get self (Variables|Parameters|GetHealthCooldownDuration) (CallFunction|GetTickRate)))
        (:then_1
          ;[0.15 0.15 0.15 0.5] Health Regen Timer Object
          (bind _returnvalue_2 (Game|ConstructObjectfromClass "/Script/TBTDungeonCrawler.TBTTimer"))
          (bind _output_get_2 (Variables|HealthRegen|SetHealthRegenObject _returnvalue_2))
          (Class|TBTTimer|Initialize _output_get_2 self 0.0 (CallFunction|GetTickRate)))
        (:then_2
          ;[0.15 0.15 0.15 0.5] Bind events for health cooldown and regen
          (if (not (Variables|Parameters|GetDisableHealthRegen))
            (EventDispatchers|BindEventtoOnTimerFinished (Variables|HealthRegen|GetHealthCooldownObject) (EventDispatchers|CreateEvent :!event Custom|BeginHealthRegen))
            (EventDispatchers|BindEventtoOnTimerTick (Variables|HealthRegen|GetHealthRegenObject) (EventDispatchers|CreateEvent :!event Custom|HandleHealthRegen))
            (EventDispatchers|BindEventtoOnTimerFinished (Variables|HealthRegen|GetHealthRegenObject) (EventDispatchers|CreateEvent :!event Custom|FinishHealthRegen))))))
    (:then_1
      (Utilities|FlowControl|Sequence
        (:then_0
          ;[0.15 0.15 0.15 0.5] Cooldown Timer Object
          (bind _returnvalue_3 (Game|ConstructObjectfromClass "/Script/TBTDungeonCrawler.TBTTimer"))
          (bind _output_get_3 (Variables|StaminaRegen|SetStaminaCooldownObject _returnvalue_3))
          (Class|TBTTimer|Initialize _output_get_3 self (Variables|Parameters|GetStaminaCooldownDuration) (CallFunction|GetTickRate)))
        (:then_1
          ;[0.15 0.15 0.15 0.5] Health Regen Timer Object
          (bind _returnvalue_4 (Game|ConstructObjectfromClass "/Script/TBTDungeonCrawler.TBTTimer"))
          (bind _output_get_4 (Variables|StaminaRegen|SetStaminaRegenObject _returnvalue_4))
          (Class|TBTTimer|Initialize _output_get_4 self 0.0 (CallFunction|GetTickRate)))
        (:then_2
          ;[0.15 0.15 0.15 0.5] Bind events for health cooldown and regen
          (EventDispatchers|BindEventtoOnTimerFinished (Variables|StaminaRegen|GetStaminaCooldownObject) (EventDispatchers|CreateEvent :!event Custom|BeginStaminaRegen))
          (EventDispatchers|BindEventtoOnTimerTick (Variables|StaminaRegen|GetStaminaRegenObject) (EventDispatchers|CreateEvent :!event Custom|HandleStaminaRegen))
          (EventDispatchers|BindEventtoOnTimerFinished (Variables|StaminaRegen|GetStaminaRegenObject) (EventDispatchers|CreateEvent :!event Custom|FinishStaminaRegen)))))))

(fn IsAlive
  (return (> (Variables|Default|GetHealthCurrent) 0.0)))