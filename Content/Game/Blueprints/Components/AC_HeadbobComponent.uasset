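; Actor component that adds walking headbob to a Character through camera shake.
; On BeginPlay it casts its owner to Character and starts a looping timer at its tick rate in place of per-frame Tick.
; When headbob is enabled, each timer tick starts the walk shake on player controller 0 if the owner has velocity and CanJump is true.
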(event Custom|HeadbobFixedTick
  (Variables|Default|GetCharacter
    (:then
      (if (Variables|Parameters|GetEnableHeadbob)
        ;[1 0.000356 0.09602] Replace with enum
        (if (CallFunction|ShouldWalkBob)
          (Game|Feedback|ClientStartCameraShake (Game|GetPlayerController 0) (Variables|Parameters|GetWalkShake) 1.0 "CameraLocal" "0, 0, 0"))))
    (:else
      (Development|PrintString "Component owner is not of type Character"))))

(event EventBeginPlay
  (bind _ascharacter (Utilities|Casting|CastToCharacter (Components|GetOwner)))
  (Variables|Default|SetCharacter _ascharacter)
  (bind _returnvalue (Utilities|Time|SetTimerbyEvent (EventDispatchers|CreateEvent :!event Custom|HeadbobFixedTick) (CallFunction|GetTickRate) true))
  (Variables|Default|SetHeadbobTimerRef _returnvalue))

(fn ShouldWalkBob
  (return (and (> (Math|Vector|VectorLength (Transformation|GetVelocity (Variables|Default|GetCharacter))) 0.0) (Character|CanJump (Variables|Default|GetCharacter)))))