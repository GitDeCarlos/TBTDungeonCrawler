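; BP_PPV is a post-process actor that applies the player's saved graphics preferences for bloom and motion blur.
; On ApplySaveData, it reads the user settings from the Game Instance and sets each effect to its configured strength if enabled, or zero if disabled.
; PullSaveData and PushSaveData only return false, so the actor stores no save data of its own.
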(event EventApplySaveData
  (bind _usersettingssave (Class|BPIGI|GetUserSettingsSave(Message) (Game|GetGameInstance)))
  (Utilities|Struct|SetmembersinPostProcessSettings (Variables|/Script/Engine.PostProcessComponent|GetSettings (Variables|Default|GetPostProcess)) (Math|Float|SelectFloat (Variables|Default|GetBloomIntensity) 0.0 (.Bloom (Utilities|Struct|BreakS_GraphicsSettings (Variables|/Game/Game/Systems/SaveData/SG_UserSettings.SG_UserSettings_C|GetGraphicsSettings _usersettingssave)))) (Math|Float|SelectFloat (Variables|Default|GetMotionBlurStrength) 0.0 (.MotionBlur (Utilities|Struct|BreakS_GraphicsSettings (Variables|/Game/Game/Systems/SaveData/SG_UserSettings.SG_UserSettings_C|GetGraphicsSettings _usersettingssave))))))

(fn ConstructionScript)

(fn PullSaveData
  (return false))

(fn PushSaveData
  (return false))