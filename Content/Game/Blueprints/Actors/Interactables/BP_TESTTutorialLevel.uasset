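; Lockable interactable, named as a tutorial-level test, that swings a separate Bridge actor open and closed like a door.
; When locked, Interact checks the Source's inventory for Key, then either unlocks without opening or prints a not-found message.
; When unlocked, it plays a sound and toggles a timeline that drives the Bridge's yaw, reversing to close.
; Getters expose action type, hold settings and widget location, with the action type following the state.
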(event Custom|OpenDoor
  (bind _bridge (Variables|Default|GetBridge))
  (bind _returnvalue (Transformation|GetActorRotation _bridge))
  (Variables|Default|SetIsOpen true)
  (Variables|Default|SetInteractionActionType "NewEnumerator2")
  (bind _deltaz (Timeline|DoorTL Play)
    (:Update
      (Transformation|SetActorRotation _bridge (Math|Rotator|MakeRotator (.roll _returnvalue) (.pitch _returnvalue) _deltaz)))))

(event Custom|CloseDoor
  (bind _bridge (Variables|Default|GetBridge))
  (bind _returnvalue (Transformation|GetActorRotation _bridge))
  (Variables|Default|SetIsOpen false)
  (Variables|Default|SetInteractionActionType "NewEnumerator1")
  (bind _deltaz (Timeline|DoorTL Reverse)
    (:Update
      (Transformation|SetActorRotation _bridge (Math|Rotator|MakeRotator (.roll _returnvalue) (.pitch _returnvalue) _deltaz)))))

(event Custom|Unlock
  (Variables|Default|SetIsLocked false)
  (Variables|Default|SetInteractionActionType "NewEnumerator1"))

(event EventInteract
  (params (Source :type Actor%20Object%20Reference))
  (if (Variables|Default|GetIsLocked)
    (bind _result (Class|BPIPlayerFunctions|CheckInventoryforItem(Message) Source (Variables|Default|GetKey)))
    (if _result
      (CallFunction|Unlock)
      (else
        (Development|PrintString (Utilities|String|ToString(Text) (Utilities|Text|FormatText "{keyname} not found" (Variables|Default|GetKey))))))
    (else
      (if (Variables|Default|GetIsOpen)
        (CallFunction|CloseDoor)
        (else
          (CallFunction|OpenDoor)))
      (Audio|PlaySound2D (Variables|Default|GetInteractSound) 1.0 1.0 0.0 0 0))))

(fn ConstructionScript)

(fn GetHoldDuration
  (return (Variables|Default|GetHoldDuration)))

(fn GetInteractionActionType
  (return (Variables|Default|GetInteractionActionType)))

(fn GetInteractionType
  (return (Variables|Default|GetInteractionType)))

(fn GetItemName
  (return ""))

(fn GetWidgetOffset
  (return (Transformation|GetWorldLocation (Variables|Default|GetInteractCollider))))