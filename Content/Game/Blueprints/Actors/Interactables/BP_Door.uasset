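; BP_Door is an interactable door that toggles between open and closed each time it is used, playing a non-spatial 2D sound.
; A single timeline plays forward to open and reverses to close, driving the door mesh's relative yaw.
; Interaction query functions report a zero hold duration, a fixed action type and a configurable interaction type.
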(event Custom|OpenDoor
  (Variables|Default|SetIsOpen true)
  (bind _deltaz (Timeline|DoorTL Play)
    (:Update
      (Transformation|SetRelativeRotation (Variables|Default|GetDoorMesh) (Math|Rotator|MakeRotator 0.0 0.0 _deltaz) false false))))

(event Custom|CloseDoor
  (Variables|Default|SetIsOpen false)
  (bind _deltaz (Timeline|DoorTL Reverse)
    (:Update
      (Transformation|SetRelativeRotation (Variables|Default|GetDoorMesh) (Math|Rotator|MakeRotator 0.0 0.0 _deltaz) false false))))

(event EventInteract
  (params (Source :type Actor%20Object%20Reference))
  (if (Variables|Default|GetIsOpen)
    (CallFunction|CloseDoor)
    (else
      (CallFunction|OpenDoor)))
  (Audio|PlaySound2D (Variables|Default|GetInteractSound) 1.0 1.0 0.0 0 0))

(fn ConstructionScript)

(fn GetHoldDuration
  (return 0.0))

(fn GetInteractionActionType
  (return "NewEnumerator0"))

(fn GetInteractionType
  (return (Variables|Default|GetInteractionType)))