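; BP_Key is an interactable key pickup that adds itself to the interacting actor's inventory by item name.
; On Interact it sends an inventory message to the source, prints a confirmation, plays a pickup sound and destroys itself.
; The construction script tints a dynamic material with LockColor, and getter functions expose interaction type, action, hold duration, name and the collider location for widget placement.
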(event EventInteract
  (params (Source :type Actor%20Object%20Reference))
  (Class|BPIPlayerFunctions|AddtoInventory(Message) Source (Variables|Default|GetItemName) self)
  (Development|PrintString (Utilities|String|ToString(Text) (Utilities|Text|FormatText "Added {ItemName} to Inventory" (Variables|Default|GetItemName))))
  (Audio|PlaySound2D (Variables|Default|GetPickUpSound) 1.0 1.0 0.0 0 0)
  (Actor|DestroyActor))

(fn ConstructionScript
  (bind _lockcolor (Variables|Default|GetLockColor))
  (bind _returnvalue (Rendering|Material|CreateDynamicMaterialInstance (Variables|Default|GetMesh) 0 (Variables|Default|GetBaseMaterial) "None" :!class /Script/Engine.PrimitiveComponent))
  (Variables|Default|SetDynamicMaterial _returnvalue)
  (Rendering|Material|SetVectorParameterValue (Variables|Default|GetDynamicMaterial) "Color1" _lockcolor :!class /Script/Engine.MaterialInstanceDynamic)
  (Rendering|Material|SetVectorParameterValue (Variables|Default|GetDynamicMaterial) "Color2" _lockcolor :!class /Script/Engine.MaterialInstanceDynamic)
  (Audio|Parameter|SetFloatParameter (Variables|Default|GetDynamicMaterial) "Favor" 0.0 :!class /Script/AudioExtensions.AudioParameterControllerInterface)
  (Audio|Parameter|SetFloatParameter (Variables|Default|GetDynamicMaterial) "Sharpness" 0.0 :!class /Script/AudioExtensions.AudioParameterControllerInterface))

(fn GetHoldDuration
  (return (Variables|Default|GetHoldDuration)))

(fn GetInteractionActionType
  (return (Variables|Default|GetInteractionActionType)))

(fn GetInteractionType
  (return (Variables|Default|GetInteractionType)))

(fn GetItemName
  (return (Variables|Default|GetItemName)))

(fn GetWidgetOffset
  (return (Transformation|GetWorldLocation (Variables|Default|GetInteractCollider))))