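; BP_PickUpItems is an interactable world item that the player picks up into their inventory.
; On Interact it sends AddToInventoryMessage with its name and itself to the source, prints a confirmation, plays a 2D pickup sound and destroys itself.
; Getter functions expose its name, hold duration, interaction and action types, and use the InteractCollider's world location as the widget offset.
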(event EventInteract
  (params (Source :type Actor%20Object%20Reference))
  (Class|BPIPlayerFunctions|AddtoInventory(Message) Source (Variables|Default|GetItemName) self)
  (Development|PrintString (Utilities|String|ToString(Text) (Utilities|Text|FormatText "Added {ItemName} to Inventory" (Variables|Default|GetItemName))))
  (Audio|PlaySound2D (Variables|Default|GetPickUpSound) 1.0 1.0 0.0 0 0)
  (Actor|DestroyActor))

(fn ConstructionScript)

(fn GetHoldDuration
  (return (Variables|Default|GetHoldDuration)))

(fn GetInteractionActionType
  (return (Variables|Default|GetInteractionActionType)))

(fn GetInteractionType
  (return (Variables|Default|GetInteractionType)))

(fn GetItemName
  (return (Variables|Default|GetItemName)))

(fn GetWidgetOffset
  (return (Transformation|GetWorldLocation (Variables|Default|GetInteractCollider))))