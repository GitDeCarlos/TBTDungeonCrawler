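; BP_HealthPickup is an interactable pickup actor that offers Health to a player.
; On BeginPlay it sets its life span when Lifespan is positive.
; Overlap on CollectionCollider checks the other actor for BPI_PlayerFunctions and sends it AddHealthPickupMessage with the Health value and itself as Source.
; The pickup does not apply health or destroy itself on collection, leaving the response to the receiver.
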(event OnComponentBeginOverlap(CollectionCollider)
  (params (OverlappedComponent :type Primitive%20Component%20Object%20Reference) (OtherActor :type Actor%20Object%20Reference) (OtherComp :type Primitive%20Component%20Object%20Reference) (OtherBodyIndex :type Integer) (bFromSweep :type Boolean) (SweepResult :type Hit%20Result%20Structure%20%28by%20ref%29))
  (if (Utilities|DoesObjectImplementInterface OtherActor "/Game/Game/Blueprints/Interfaces/BPI_PlayerFunctions.BPI_PlayerFunctions_C")
    (Class|BPIPlayerFunctions|AddHealthPickup(Message) OtherActor (Variables|Parameters|GetHealth) self)))

(event EventBeginPlay
  (if (> (Variables|Parameters|GetLifespan) 0.0)
    (Actor|SetLifeSpan (Variables|Parameters|GetLifespan))))

(fn ConstructionScript)