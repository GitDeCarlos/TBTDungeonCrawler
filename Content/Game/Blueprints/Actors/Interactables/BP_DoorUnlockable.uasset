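; Interactable double door that can be locked, opening once the interacting source's inventory holds the matching key, and toggling open and closed thereafter.
; A timeline rotates both leaves in opposite yaw and reverses to close, while open state updates the interaction action type.
; The construction script gives both meshes a shared dynamic material colored by initial lock state.
; Getter functions supply interaction type, hold duration and widget location.
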(event Custom|OpenDoor
  (Variables|Default|SetIsOpen true)
  (Variables|Default|SetInteractionActionType "NewEnumerator2")
  (bind _deltaz (Timeline|DoorTL Play)
    (:Update
      (Transformation|SetRelativeRotation (Variables|Default|GetL_DoorMesh) (Math|Rotator|MakeRotator 0.0 0.0 _deltaz) false false)
      (Transformation|SetRelativeRotation (Variables|Default|GetR_DoorMesh) (Math|Rotator|MakeRotator 0.0 0.0 (* _deltaz -1.0)) false false))))

(event Custom|CloseDoor
  (Variables|Default|SetIsOpen false)
  (Variables|Default|SetInteractionActionType "NewEnumerator1")
  (bind _deltaz (Timeline|DoorTL Reverse)
    (:Update
      (Transformation|SetRelativeRotation (Variables|Default|GetL_DoorMesh) (Math|Rotator|MakeRotator 0.0 0.0 _deltaz) false false)
      (Transformation|SetRelativeRotation (Variables|Default|GetR_DoorMesh) (Math|Rotator|MakeRotator 0.0 0.0 (* _deltaz -1.0)) false false))))

(event Custom|Unlock
  (Variables|Default|SetIsLocked false)
  (CallFunction|OpenDoor)
  (Variables|Default|SetInteractionActionType "NewEnumerator2"))

(event EventInteract
  (params (Source :type Actor%20Object%20Reference))
  (if (Variables|Default|GetIsLocked)
    (bind _result (Class|BPIPlayerFunctions|CheckInventoryforItem(Message) Source (Variables|Default|GetKey)))
    (if _result
      (CallFunction|Unlock)
      (else
        (Development|PrintString (Utilities|String|ToString(Text) (Utilities|Text|FormatText "{keyname} not found" (Variables|Default|GetKey))))))
    (else
      (if (Variables|Default|GetIsOpen)
        (CallFunction|CloseDoor)
        (else
          (CallFunction|OpenDoor)))
      (Audio|PlaySound2D (Variables|Default|GetInteractSound) 1.0 1.0 0.0 0 0))))

(fn ConstructionScript
  (bind _returnvalue (Rendering|Material|CreateDynamicMaterialInstance (Variables|Default|GetL_DoorMesh) 0 (Variables|Default|GetBaseMaterial) "None" :!class /Script/Engine.PrimitiveComponent))
  (bind _output_get (Variables|Default|SetDynamicMaterial _returnvalue))
  (Rendering|Material|SetMaterial (Variables|Default|GetR_DoorMesh) 0 _output_get)
  (Rendering|Material|SetVectorParameterValue (Variables|Default|GetDynamicMaterial) "Color1" (select (Variables|Default|GetIsLocked) (Variables|Default|GetLockColor) "(R=0.000000,G=1.000000,B=0.000000,A=1.000000)") :!class /Script/Engine.MaterialInstanceDynamic)
  (Rendering|Material|SetVectorParameterValue (Variables|Default|GetDynamicMaterial) "Color2" "(R=0.029556,G=0.036889,B=0.033104,A=1.000000)" :!class /Script/Engine.MaterialInstanceDynamic)
  (Audio|Parameter|SetFloatParameter (Variables|Default|GetDynamicMaterial) "Favor" 0.0 :!class /Script/AudioExtensions.AudioParameterControllerInterface)
  (Audio|Parameter|SetFloatParameter (Variables|Default|GetDynamicMaterial) "Sharpness" 0.0 :!class /Script/AudioExtensions.AudioParameterControllerInterface))

(fn GetHoldDuration
  (return (Variables|Default|GetHoldDuration)))

(fn GetInteractionActionType
  (return (Variables|Default|GetInteractionActionType)))

(fn GetInteractionType
  (return (Variables|Default|GetInteractionType)))

(fn GetItemName
  (return ""))

(fn GetWidgetOffset
  (return (Transformation|GetWorldLocation (Variables|Default|GetInteractCollider))))