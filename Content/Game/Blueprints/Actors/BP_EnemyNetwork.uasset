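; BP_EnemyNetwork is an actor that links a set of enemies so they can be alerted as a group.
; On BeginPlay it registers itself with each valid member through a SetEnemyNetwork message.
; AlertNetwork relays a target actor to every valid member as a RequestAlert message.
; The construction script draws debug lines from the network actor to each member to visualize the links.
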(event Custom|AlertNetwork
  (params (TargetActor :type Actor%20Object%20Reference))
  (for _array_element (Variables|Default|GetMembers)
    (Utilities|IsValid _array_element
      (:Is%20Valid
        (Class|BPIEnemyAI|RequestAlert(Message) _array_element TargetActor)))))

(event EventBeginPlay
  (for _array_element (Variables|Default|GetMembers)
    (Utilities|IsValid _array_element
      (:Is%20Valid
        (Class|BPIEnemyAI|SetEnemyNetwork(Message) _array_element self)))))

(fn ConstructionScript
  (for _array_element (Variables|Default|GetMembers)
    (Rendering|Debug|DrawDebugLine (Transformation|GetActorLocation) (Transformation|GetActorLocation _array_element) (Variables|Parameters|GetLineColor) 1e+02 2.0)))