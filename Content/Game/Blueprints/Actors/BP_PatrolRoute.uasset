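; BP_PatrolRoute is an actor that defines a patrol path from the points of its Route spline.
; It returns the world position of the point at the current PatrolIndex.
; IncrementPatrolRoute steps that index by Direction, using AtEndPoint to detect the route's ends.
; At an end, a closed-loop spline resets to the first point, while an open one flips Direction to ping-pong back.
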(fn ConstructionScript)

(fn GetSplinePointasWorldPosition
  (return (Spline|GetLocationatSplinePoint (Variables|Default|GetRoute) (Variables|Default|GetPatrolIndex) "World")))

(fn IncrementPatrolRoute
  (Utilities|FlowControl|Sequence
    (:then_0
      (if (CallFunction|AtEndPoint)
        (if (Class|SplineComponent|IsClosedLoop (Variables|Default|GetRoute))
          (Variables|Default|SetPatrolIndex 0)
          (return)
          (else
            (Utilities|NegateInt (Variables|Default|GetDirection))))))
    (:then_1
      (Variables|Default|SetPatrolIndex (+ (Variables|Default|GetPatrolIndex) (Variables|Default|GetDirection))))))

(fn AtEndPoint
  (return (or (and (== (Variables|Default|GetPatrolIndex) (- (Spline|GetNumberOfSplinePoints (Variables|Default|GetRoute)) 1)) (== (Variables|Default|GetDirection) (Variables|Constants|GetDIR_POS))) (and (== (Variables|Default|GetPatrolIndex) 0) (== (Variables|Default|GetDirection) (Variables|Constants|GetDIR_NEG))))))