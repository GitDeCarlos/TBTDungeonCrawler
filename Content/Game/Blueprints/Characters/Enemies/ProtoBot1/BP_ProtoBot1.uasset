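; BP_ProtoBot1 is a prototype enemy bot character that exposes state, patrol, movement and combat functions, likely for its AI controller AIC_ProtoBot1.
; Attack requests trigger MeleeComponent between begin and finish callbacks, while alert requests wait a random moment before switching a Passive controller to attacking the target.
; Helpers swap alert materials, set walk speed and return the patrol route and enemy network.
; StatusComponent death shows a message, unpossesses, disables capsule collision, then destroys the actor.
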(event OnDeath(StatusComponent)
  (Utilities|NewinWorldMessage "Dead" (Transformation|GetActorLocation) "ForDuration" "(R=1.000000,G=0.000356,B=0.096022,A=1.000000)" 2.0
    (:OutputPin
      (Utilities|FlowControl|Delay 0.2)
      (Pawn|UnPossess (AI|GetAIController self))
      (Collision|SetCollisionEnabled (Variables|Collision|GetCapsuleComponent) "NoCollision")
      (Utilities|FlowControl|Delay 6e+01)
      (Actor|DestroyActor))))

(event OnHealthChanged(StatusComponent)
  (params (CurrentHealth :type Float%20%28double-precision%29) (MaxHealth :type Float%20%28double-precision%29)))

(event Custom|Attack
  (Default|CallOnBeginAttack)
  (Default|MeleeAttack (Variables|Default|GetMeleeComponent))
  (Utilities|FlowControl|Delay (Variables|Parameters|GetAttackDelay))
  (Default|CallOnFinishAttack))

(event EventRequestAlert
  (params (TargetActor :type Actor%20Object%20Reference))
  (Utilities|FlowControl|Delay (Math|Random|RandomFloat))
  (bind _asaic_proto_bot_1 (Utilities|Casting|CastToAIC_ProtoBot1 (AI|GetAIController self)))
  (switch Utilities|FlowControl|Switch|SwitchonE_AIState (Default|GetCurrentState _asaic_proto_bot_1)
    (:NewEnumerator0
      (Default|SetStateasAttacking _asaic_proto_bot_1 TargetActor))))

(fn ConstructionScript)

(fn SetMaterial
  (params (InCombatState :type Boolean))
  (bind _mesh (Variables|Character|GetMesh))
  (if InCombatState
    (Rendering|Material|SetMaterial _mesh 0 (Variables|Default|GetAlertMaterial))
    (else
      (Rendering|Material|SetMaterial _mesh 0 (Variables|Default|GetDefaultMaterial)))))

(fn GetAIState
  (return "NewEnumerator0"))

(fn GetEnemyNetwork
  (return (Variables|AI|GetEnemyNetwork)))

(fn GetPatrolRoute
  (return (Variables|AI|GetPatrolRoute)))

(fn IsAlive
  (bind _result (Default|IsAlive (Variables|Default|GetStatusComponent)))
  (return _result))

(fn RequestAttack
  (CallFunction|Attack)
  (return (Variables|Parameters|GetAttackDelay)))

(fn SetMovementSpeed
  (params (Speed :type E_MovementSpeed%20Enum :default "NewEnumerator0"))
  (bind _output_get (Variables|/Script/Engine.CharacterMovementComponent|SetMaxWalkSpeed (Variables|Character|GetCharacterMovement) (Utilities|Select :Index Speed :NewEnumerator0 0.0 :NewEnumerator1 (Variables|Parameters|GetMaxWalkingSpeed) :NewEnumerator2 (Variables|Parameters|GetMaxRunningSpeed))))
  (return _output_get))