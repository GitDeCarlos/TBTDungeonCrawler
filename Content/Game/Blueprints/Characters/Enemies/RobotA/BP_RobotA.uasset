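; BP_RobotA is an enemy robot character that exposes patrol route, enemy network, alive state, movement speed and attack functions.
; Alert requests wait a random delay, then switch a Passive AIC_RobotA controller to Combat on the target.
; On StatusComponent death it unpossesses, ragdolls with an impulse, expires after a delay and may spawn a drop.
; Attack requests play a montage, while GetAIState always returns Passive instead of querying the controller.
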(event OnDeath(StatusComponent)
  (bind _returnvalue (Transformation|GetActorLocation))
  (bind _self self)
  (bind _mesh (Variables|Character|GetMesh))
  (Utilities|NewinWorldMessage "Dead" (Transformation|GetActorLocation) "ForDuration" "(R=1.000000,G=0.101570,B=0.275602,A=1.000000)" 2.0
    (:OutputPin
      (Pawn|UnPossess (AI|GetAIController _self))
      (Collision|SetCollisionEnabled (Variables|Collision|GetCapsuleComponent) "NoCollision")
      (Physics|SetSimulatePhysics _mesh true)
      (Physics|AddImpulse _mesh "-100.000000,-500.000000,800.000000" "" true)
      (Actor|SetLifeSpan _self 3e+01)
      (if (CallFunction|CheckChance 0.5 1.0)
        (Game|SpawnActorfromClass (Variables|Default|GetDeathDrop) (Math|Transform|MakeTransform (Math|Vector|MakeVector (.x _returnvalue) (.y _returnvalue) 0.0) "0, 0, 0" "1.000000,1.000000,1.000000") "Undefined" "MultiplyWithRoot" 0 4.0 1e+01 0)))))

(event OnHealthChanged(StatusComponent)
  (params (CurrentHealth :type Float%20%28double-precision%29) (MaxHealth :type Float%20%28double-precision%29)))

(event EventRequestAlert
  (params (TargetActor :type Actor%20Object%20Reference))
  (Utilities|FlowControl|Delay (Math|Random|RandomFloat))
  (bind _asaic_robot_a (Utilities|Casting|CastToAIC_RobotA (AI|GetAIController self)))
  (switch Utilities|FlowControl|Switch|SwitchonE_AIState (Default|GetCurrentState _asaic_robot_a)
    (:NewEnumerator0
      (Default|SetStateasCombat _asaic_robot_a TargetActor))))

(event EventSetEnemyNetwork
  (params (EnemyNetworkObject :type BP%20Enemy%20Network%20Object%20Reference))
  (Variables|AI|SetEnemyNetwork EnemyNetworkObject))

(fn ConstructionScript)

(fn GetAIState
  (return "NewEnumerator0"))

(fn GetEnemyNetwork
  (return (Variables|AI|GetEnemyNetwork)))

(fn GetPatrolRoute
  (return (Variables|AI|GetPatrolRoute)))

(fn IsAlive
  (bind _result (Default|IsAlive (Variables|Default|GetStatusComponent)))
  (return _result))

(fn RequestAttack
  (Utilities|NewinWorldMessage "Attack request received" (Transformation|GetActorLocation) "ForDuration" "(R=1.000000,G=1.000000,B=1.000000,A=1.000000)" 2.0
    (:OutputPin
      (bind _returnvalue (Animation|PlayAnimMontage (Variables|Default|GetAttackMontage) 1.0 "None"))
      (return _returnvalue))))

(fn SetMovementSpeed
  (params (Speed :type E_MovementSpeed%20Enum :default "NewEnumerator0"))
  (bind _output_get (Variables|/Script/Engine.CharacterMovementComponent|SetMaxWalkSpeed (Variables|Character|GetCharacterMovement) (Utilities|Select :Index Speed :NewEnumerator0 0.0 :NewEnumerator1 (Variables|Parameters|GetWalkingSpeed) :NewEnumerator2 (Variables|Parameters|GetRunningSpeed))))
  (return _output_get))