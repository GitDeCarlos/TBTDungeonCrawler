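; Main player controller that sets up local input and the game UI layer, and handles pausing.
; On BeginPlay it adds the default, mouse look and dungeon crawler mapping contexts, creates the UIL_Game layer and sets game-only input.
; IA_Pause toggles pause, switching game pause state, input mode and cursor while pushing or popping the pause widget on that layer.
; The pause widget's Continue click is bound when pushed.
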(event Input|EnhancedActionEvents|EnhancedInputActionIA_Pause
  (params (ActionValue :type Boolean) (ElapsedSeconds :type Float%20%28double-precision%29) (TriggeredSeconds :type Float%20%28double-precision%29) (InputAction :type Input%20Action%20Object%20Reference :default "/Game/Game/Systems/Input/Actions/IA_Pause.IA_Pause"))
  (:Started
    (CallFunction|TogglePause)))

(event EventBeginPlay
  (bind _self self)
  (if (Pawn|IsLocalPlayerController)
    (Utilities|FlowControl|Sequence
      (:then_0
        (CallFunction|AddInputMapping _self "/Game/Game/Systems/Input/IMC_Default.IMC_Default")
        (CallFunction|AddInputMapping _self "/Game/Game/Systems/Input/IMC_MouseLook.IMC_MouseLook")
        (CallFunction|AddInputMapping _self "/Game/Game/Systems/Input/IMC_DungeonCrawler.IMC_DungeonCrawler"))
      (:then_1
        (bind _returnvalue (UserInterface|CreateWidget "/Game/Game/Systems/Menu/UIL_Game.UIL_Game_C" (Game|GetPlayerController 0)))
        (bind _output_get (Variables|Default|SetUILayerRef _returnvalue))
        (UserInterface|Viewport|AddtoViewport _output_get 0))
      (:then_2
        (Input|SetInputModeGameOnly self false)))))

(fn ConstructionScript)

(fn TogglePause
  (if (Variables|Default|GetInPauseScreen)
    (CallFunction|UnpauseGame)
    (else
      (CallFunction|PauseGame))))

(fn PauseGame
  (Utilities|FlowControl|Sequence
    (:then_0
      (Game|SetGamePaused true)
      (Variables|Default|SetInPauseScreen true)
      (Input|SetInputModeGameandUI self (Variables|Default|GetUILayerRef) "DoNotLock" true false)
      (Variables|Default|SetbShowMouseCursor true))
    (:then_1
      (bind _output_get (Default|PushWidget (Variables|Default|GetUILayerRef) "/Game/Game/UI/Screens/UI_Game_Pause.UI_Game_Pause_C"))
      (bind _asui_game_pause (Utilities|Casting|CastToUI_Game_Pause _output_get)
        (:then
          (EventDispatchers|BindEventtoOnContinueClicked _asui_game_pause (EventDispatchers|CreateEvent :!event UnpauseGame)))
        (:CastFailed
          (Development|PrintString "ERROR: CAST FAILED" true true "(R=1.000000,G=0.000356,B=0.096022,A=1.000000)"))))))

(fn UnpauseGame
  (Utilities|FlowControl|Sequence
    (:then_0
      (Game|SetGamePaused false)
      (Variables|Default|SetInPauseScreen false)
      (Input|SetInputModeGameOnly self false)
      (Variables|Default|SetbShowMouseCursor false))
    (:then_1
      (Default|PopWidget (Variables|Default|GetUILayerRef)))))