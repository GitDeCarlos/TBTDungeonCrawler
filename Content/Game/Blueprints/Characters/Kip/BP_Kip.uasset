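; BP_Kip is a character that can be picked up as an inventory item and can also die.
; Its interaction interface reports the name "kip" and zero hold duration, and Interact sends the item to the source's inventory, prints a message, plays a sound and destroys the actor.
; A StatusComponent answers the alive check, and its death event shows a red "Ow" in-world message at the actor's location.
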(event OnDeath(StatusComponent)
  (Utilities|NewinWorldMessage "Ow" (Transformation|GetActorLocation) "ForDuration" "(R=1.000000,G=0.000356,B=0.096022,A=1.000000)" 2.0))

(event EventInteract
  (params (Source :type Actor%20Object%20Reference))
  (Class|BPIPlayerFunctions|AddtoInventory(Message) Source (Variables|Default|GetItemName) self)
  (Development|PrintString (Utilities|String|ToString(Text) (Utilities|Text|FormatText "Added {ItemName} to Inventory" (Variables|Default|GetItemName))))
  (Audio|PlaySound2D (Variables|Default|GetPickUpSound) 1.0 1.0 0.0 0 0)
  (Actor|DestroyActor))

(fn ConstructionScript)

(fn GetHoldDuration
  (return 0.0))

(fn GetInteractionActionType
  (return "NewEnumerator0"))

(fn GetInteractionType
  (return "NewEnumerator0"))

(fn GetItemName
  (return "kip"))

(fn GetWidgetOffset
  (return "0, 0, 0"))

(fn IsAlive
  (bind _result (Default|IsAlive (Variables|Default|GetStatusComponent)))
  (return _result))